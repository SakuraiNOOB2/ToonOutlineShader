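; BP_Door is a door actor that swings open through a timeline and closes itself afterwards.
; OpenDoor plays the DoorOpen timeline only when IsOpen is already true, lerping the Door's world rotation toward a 90-degree turn.
; On finish it waits briefly, then clears IsOpen and reverses the timeline through CloseDoor.
; IsOpen starts false and nothing in this Blueprint sets it true.
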(event Custom|OpenDoor
  (Components|Timeline|SetPlayRate (Variables|Default|GetDoorOpen) (/ 1.0 1.0))
  (if (Variables|Default|GetisOpen)
    (bind _doorrotationz (Timeline|DoorOpen PlayFromStart)
      (:Update
        (Transformation|SetWorldRotation (Variables|Default|GetDoor) (Math|Rotator|Lerp(Rotator) "0, 0, 0" "0.000000,90.000000,0.000000" _doorrotationz true) false false))
      (:Finished
        (Utilities|FlowControl|Delay 0.5)
        (if (Variables|Default|GetisOpen)
          (Variables|Default|SetisOpen false)
          (CallFunction|CloseDoor))))))

(event Custom|CloseDoor
  (bind _doorrotationz (Timeline|DoorOpen ReverseFromEnd)
    (:Update
      (Transformation|SetWorldRotation (Variables|Default|GetDoor) (Math|Rotator|Lerp(Rotator) "0, 0, 0" "0.000000,90.000000,0.000000" _doorrotationz true) false false))
    (:Finished
      (Utilities|FlowControl|Delay 0.5)
      (if (Variables|Default|GetisOpen)
        (Variables|Default|SetisOpen false)
        (CallFunction|CloseDoor)))))

(event EventBeginPlay
  (Variables|Default|SetisOpen false))

(event EventTick
  (params (DeltaSeconds :type Float%20%28single-precision%29)))

(fn ConstructionScript)